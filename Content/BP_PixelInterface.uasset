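; BP_PixelInterface creates the display widget, listens for Pixel Streaming input and provides keyboard level switching.
; On BeginPlay it finds the PixelStreamingInputComponent on the first player controller and binds its input event, printing whether the component is valid.
; Received event descriptors are only printed on screen.
; The N key swaps between Map1 and Map2, while R reloads the current map, both by switching on the level name.
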(event `self.ReceiveBeginPlay`
  (bind _returnvalue (`self.GetComponentByClass` (`GameplayStatics.GetPlayerController` 0) "/Script/PixelStreaming.PixelStreamingInputComponent"))
  (bind _returnvalue_2 (`|CreateWidget` "/Game/WBP_Display.WBP_Display_C" (`GameplayStatics.GetPlayerController` 0)))
  (`UserWidget.AddToViewport` _returnvalue_2 0)
  (`/Engine/EditorBlueprintResources/StandardMacros.IsValid` _returnvalue
    (:`Is Valid`
      (`KismetSystemLibrary.PrintString` "Pixel streaming component valid" true true (struct :`G` 1.0 :`B` 0.089466 :`A` 1.0) 5.0)
      (set `self.PixelRef` _returnvalue)
      (add `PixelStreamingInputComponent.OnPixelStreamingInputEvent` (`self.PixelRef`) (delegate `PixelEvent`)))
    (:`Is Not Valid`
      (`KismetSystemLibrary.PrintString` "Pixel streaming component not valid" true true (struct :`R` 1.0 :`B` 0.013496 :`A` 1.0) 5.0))))

(event `PixelEvent`
  (params (Descriptor :type String))
  (`KismetSystemLibrary.PrintString` (`KismetStringLibrary.Concat_StrStr` "Event recieved: " Descriptor) true true (struct :`R` 1.0 :`B` 0.879078 :`A` 1.0)))

(event `Key|N`
  (params (Key :type "Key Structure"))
  (:`Pressed`
    (bind _returnvalue (`GameplayStatics.GetCurrentLevelName` true))
    (switch `string` _returnvalue
      (:`Map1`
        (`GameplayStatics.OpenLevel` "Map2" :!label _label))
      (:`Map2`
        (`GameplayStatics.OpenLevel` "Map1" :!label _label_2)))))

(event `Key|R`
  (params (Key :type "Key Structure"))
  (:`Pressed`
    (bind _returnvalue (`GameplayStatics.GetCurrentLevelName` true))
    (switch `string` _returnvalue
      (:`Map1`
        (goto _label_2))
      (:`Map2`
        (goto _label)))))

(fn `UserConstructionScript`)